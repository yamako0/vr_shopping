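; Player pawn that operates an in-world UI widget through a right motion controller's WidgetInteraction component.
; Touch_B or right mouse flip-flops the UI, switching input mode, cursor and pointer activation along with it.
; While the UI shows, Tick draws a debug line as a pointer ray, and Trigger acts as a left mouse click.
; GetSpawnLocation returns the SpawnPoint actor's location when valid.
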(event EventBeginPlay
  (|CallParentFunction))

(event Collision|EventActorBeginOverlap
  (params (OtherActor :type Actor%20Object%20Reference)))

(event EventTick
  (params (DeltaSeconds :type Float%20%28single-precision%29))
  (bind _rightcontroller (Variables|Default|GetRightController))
  (bind _widgetinteraction (Variables|/Game/VirtualRealityBP/Blueprints/BP_MotionController.BP_MotionController_C|GetWidgetInteraction _rightcontroller))
  (bind _returnvalue (Transformation|GetWorldLocation _widgetinteraction))
  (|CallParentFunction DeltaSeconds)
  ;[0 0 0] Draw Line
  (if (Variables|Default|GetCanSeeUI)
    (Rendering|Debug|DrawDebugLine _returnvalue (+ _returnvalue (* (Math|Vector|GetForwardVector _widgetinteraction) 5e+02)) "(R=1.000000,G=0.263967,B=0.000000,A=1.000000)" 0.0 0.25)))

(event Input|ActionEvents|InputActionTouch_B
  (params (Key :type Key%20Structure :default "AnyKey"))
  (bind _returnvalue (Game|GetPlayerController 0))
  (bind _ui (Variables|Default|GetUI))
  (bind _rightcontroller (Variables|Default|GetRightController))
  (bind _widgetinteraction (Variables|/Game/VirtualRealityBP/Blueprints/BP_MotionController.BP_MotionController_C|GetWidgetInteraction _rightcontroller))
  ;[0 0 0] Switch Window
  (:Pressed
    (Utilities|FlowControl|FlipFlop
      (:A
        (Development|SetHiddeninGame _ui false false)
        (Input|SetInputModeGameandUI _returnvalue (UserInterface|GetUserWidgetObject _ui) "DoNotLock" true)
        (Variables|/Script/Engine.PlayerController|SetbShowMouseCursor _returnvalue true)
        (Components|Activation|Activate _widgetinteraction false)
        (Variables|Default|SetCanSeeUI true))
      (:B
        (Development|SetHiddeninGame _ui true false)
        (Input|SetInputModeGameOnly _returnvalue)
        (Variables|/Script/Engine.PlayerController|SetbShowMouseCursor _returnvalue false)
        (Components|Activation|Deactivate _widgetinteraction)
        (Variables|Default|SetCanSeeUI false)))))

(event Input|ActionEvents|InputActionTrigger
  (params (Key :type Key%20Structure :default "AnyKey"))
  (bind _rightcontroller (Variables|Default|GetRightController))
  (bind _widgetinteraction (Variables|/Game/VirtualRealityBP/Blueprints/BP_MotionController.BP_MotionController_C|GetWidgetInteraction _rightcontroller))
  ;[0 0 0] Trigger Adapter
  (:Pressed
    (Class|WidgetInteractionComponent|PressPointerKey _widgetinteraction "LeftMouseButton"))
  (:Released
    (Class|WidgetInteractionComponent|ReleasePointerKey _widgetinteraction "LeftMouseButton")))

(event Input|MouseEvents|RightMouseButton
  (params (Key :type Key%20Structure :default "AnyKey"))
  (bind _returnvalue (Game|GetPlayerController 0))
  (bind _ui (Variables|Default|GetUI))
  (bind _rightcontroller (Variables|Default|GetRightController))
  (bind _widgetinteraction (Variables|/Game/VirtualRealityBP/Blueprints/BP_MotionController.BP_MotionController_C|GetWidgetInteraction _rightcontroller))
  ;[0 0 0] Switch Window
  (:Pressed
    (Utilities|FlowControl|FlipFlop
      (:A
        (Development|SetHiddeninGame _ui false false)
        (Input|SetInputModeGameandUI _returnvalue (UserInterface|GetUserWidgetObject _ui) "DoNotLock" true)
        (Variables|/Script/Engine.PlayerController|SetbShowMouseCursor _returnvalue true)
        (Components|Activation|Activate _widgetinteraction false)
        (Variables|Default|SetCanSeeUI true))
      (:B
        (Development|SetHiddeninGame _ui true false)
        (Input|SetInputModeGameOnly _returnvalue)
        (Variables|/Script/Engine.PlayerController|SetbShowMouseCursor _returnvalue false)
        (Components|Activation|Deactivate _widgetinteraction)
        (Variables|Default|SetCanSeeUI false)))))

(fn ConstructionScript
  (|CallParentFunction))

(fn GetSpawnLocation
  (bind _spawnpoint (Variables|Default|GetSpawnPoint))
  (Utilities|IsValid _spawnpoint
    (:Is%20Valid
      (return (Transformation|GetActorLocation _spawnpoint)))))