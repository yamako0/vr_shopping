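; Test character that flies freely along its camera's view, ignoring collision.
; The construction script disables CharacterMovement, and the MoveForward and MoveRight axes offset the actor directly with an unswept SetActorLocation along the camera's forward and right vectors.
; Turn and LookUp feed controller yaw and pitch.
; Movement is not scaled by delta time, so its speed depends on frame rate.
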(event Input|AxisEvents|InputAxisMoveRight
  (params (AxisValue :type Float%20%28single-precision%29))
  (Transformation|SetActorLocation (+ (* (Math|Vector|GetRightVector (Transformation|GetWorldRotation (Variables|Default|GetCamera))) AxisValue) (Transformation|GetActorLocation)) false false))

(event Input|AxisEvents|InputAxisMoveForward
  (params (AxisValue :type Float%20%28single-precision%29))
  (Transformation|SetActorLocation (+ (* (Math|Vector|GetForwardVector (Transformation|GetWorldRotation (Variables|Default|GetCamera))) AxisValue) (Transformation|GetActorLocation)) false false))

(event Input|AxisEvents|InputAxisLookUp
  (params (AxisValue :type Float%20%28single-precision%29))
  (Pawn|Input|AddControllerPitchInput AxisValue))

(event Input|AxisEvents|InputAxisTurn
  (params (AxisValue :type Float%20%28single-precision%29))
  (Pawn|Input|AddControllerYawInput AxisValue))

(fn ConstructionScript
  (Pawn|Components|CharacterMovement|DisableMovement (Variables|Character|GetCharacterMovement)))