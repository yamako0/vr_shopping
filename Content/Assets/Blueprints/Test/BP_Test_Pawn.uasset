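; BP_Test_Pawn is a test pawn that flies freely and toggles an in-world or on-screen TestUI widget component.
; Axis inputs offset the actor location along camera vectors or world Z without sweep or delta-time scaling, and feed controller yaw and pitch.
; Right mouse and Touch_B share a FlipFlop that switches widget visibility, cursor and input mode.
; GetSpawnTransform returns a point ahead of the pawn with pitch zeroed.
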(event Input|ActionEvents|InputActionTouch_B
  (params (Key :type Key%20Structure :default "AnyKey"))
  (bind _returnvalue (Game|GetPlayerController 0))
  (bind _test_ui (Variables|Default|GetTest_UI))
  (:Pressed
    (Utilities|FlowControl|FlipFlop
      (:A
        (Development|SetHiddeninGame _test_ui false false)
        (Input|SetInputModeGameandUI _returnvalue (UserInterface|GetUserWidgetObject (Variables|Default|GetTest_UI)) "DoNotLock" true)
        (Variables|/Script/Engine.PlayerController|SetbShowMouseCursor _returnvalue true))
      (:B
        (Development|SetHiddeninGame _test_ui true false)
        (Input|SetInputModeGameOnly _returnvalue)
        (Variables|/Script/Engine.PlayerController|SetbShowMouseCursor _returnvalue false)))))

(event Input|AxisEvents|InputAxisMoveRight
  (params (AxisValue :type Float%20%28single-precision%29))
  ;[1 1 1] Movement
  (Transformation|SetActorLocation (+ (* (Math|Vector|GetRightVector (Variables|Default|GetCamera)) (* AxisValue (Variables|Default|GetSpeed))) (Transformation|GetActorLocation)) false false))

(event Input|AxisEvents|InputAxisMoveForward
  (params (AxisValue :type Float%20%28single-precision%29))
  ;[1 1 1] Movement
  (Transformation|SetActorLocation (+ (* (Math|Vector|GetForwardVector (Variables|Default|GetCamera)) (* AxisValue (Variables|Default|GetSpeed))) (Transformation|GetActorLocation)) false false))

(event Input|AxisEvents|InputAxisLookUp
  (params (AxisValue :type Float%20%28single-precision%29))
  ;[1 1 1] Movement
  (Pawn|Input|AddControllerPitchInput AxisValue))

(event Input|AxisEvents|InputAxisUp
  (params (AxisValue :type Float%20%28single-precision%29))
  (bind _returnvalue (Transformation|GetActorLocation))
  (bind (_x _y _z) (Math|Vector|BreakVector _returnvalue))
  ;[1 1 1] Movement
  (Transformation|SetActorLocation (Math|Vector|MakeVector _x _y (+ _z (* AxisValue 3.0))) false false))

(event Input|AxisEvents|InputAxisTurn
  (params (AxisValue :type Float%20%28single-precision%29))
  ;[1 1 1] Movement
  (Pawn|Input|AddControllerYawInput AxisValue))

(event Input|MouseEvents|RightMouseButton
  (params (Key :type Key%20Structure :default "AnyKey"))
  (bind _returnvalue (Game|GetPlayerController 0))
  (bind _test_ui (Variables|Default|GetTest_UI))
  (:Pressed
    (Utilities|FlowControl|FlipFlop
      (:A
        (Development|SetHiddeninGame _test_ui false false)
        (Input|SetInputModeGameandUI _returnvalue (UserInterface|GetUserWidgetObject (Variables|Default|GetTest_UI)) "DoNotLock" true)
        (Variables|/Script/Engine.PlayerController|SetbShowMouseCursor _returnvalue true))
      (:B
        (Development|SetHiddeninGame _test_ui true false)
        (Input|SetInputModeGameOnly _returnvalue)
        (Variables|/Script/Engine.PlayerController|SetbShowMouseCursor _returnvalue false)))))

(fn ConstructionScript)

(fn GetSpawnTransform
  (bind _returnvalue (Transformation|GetActorRotation))
  (bind (_roll _pitch _yaw) (Math|Rotator|BreakRotator _returnvalue))
  (return (Math|Transform|MakeTransform (+ (Transformation|GetActorLocation) (* (Transformation|GetActorForwardVector) 1e+02)) (Math|Rotator|MakeRotator _roll 0.0 _yaw))))